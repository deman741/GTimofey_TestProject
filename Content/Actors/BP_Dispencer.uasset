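; Item dropper actor that holds a spawned prop and releases it when activated, with iris open and close animations, material swaps and sounds.
; A prop spawns on BeginPlay, and Activate calls DropItem, which opens the dropper and disables the Box collision behind a DoOnce.
; When a physics prop leaves Box5, the dropper closes, restores collision and spawns a replacement, re-arming the drop unless DropOneTime is set.
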(event OnComponentEndOverlap(Box5)
  (params (OverlappedComponent :type Primitive%20Component%20Object%20Reference) (OtherActor :type Actor%20Object%20Reference) (OtherComp :type Primitive%20Component%20Object%20Reference) (OtherBodyIndex :type Integer))
  (bind _box (Variables|Default|GetBox))
  (bind _returnvalue (Transformation|GetWorldLocation _box))
  (Utilities|Casting|CastToBP_PhysicProp OtherActor)
  (Utilities|FlowControl|RetriggerableDelay 0.2)
  (if (Variables|Default|GetCanClose)
    (Audio|PlaySoundatLocation "/Game/Portal2Content/sounds/buttons/dropper_iris_close_01.dropper_iris_close_01" _returnvalue "0, 0, 0" 0.1 1.0 0.0 "/Game/Portal2Content/sounds/SA_Default.SA_Default" 0 0 0)
    (Rendering|Material|SetMaterial (Variables|Default|Getitem_dropper1) 0 "/Game/Portal2Content/models/Dropper/item_dropper.item_dropper")
    (Components|Animation|PlayAnimation (Variables|Default|Getitem_dropper1) "/Game/Portal2Content/models/Dropper/item_dropper_Anim_item_dropper_qc_skeleton_item_dropper_close.item_dropper_Anim_item_dropper_qc_skeleton_item_dropper_close" false)
    (Utilities|FlowControl|Delay 1.5)
    (Collision|SetCollisionEnabled (Variables|Default|GetBox) "PhysicsOnly")
    (Variables|Default|SetCanClose false)
    (Utilities|FlowControl|Sequence
      (:then_0
        (Game|SpawnActorfromClass (Variables|Default|GetPropToSpawn_0) (Math|Transform|MakeTransform (Transformation|GetWorldLocation (Variables|Default|GetDefaultSceneRoot)) "0, 0, 0" "1.000000,1.000000,1.000000") "AlwaysSpawn" "MultiplyWithRoot" 0 0))
      (:then_1
        (if (not (Variables|Default|GetDropOneTime))
          (Utilities|FlowControl|DoOnce false) ; enters at Reset
        )))))

(event Custom|DropItem
  (Utilities|FlowControl|DoOnce false
    (:Completed
      (Rendering|Material|SetMaterial (Variables|Default|Getitem_dropper1) 0 "/Game/Portal2Content/models/Dropper/item_dropper2.item_dropper2")
      (Components|Animation|PlayAnimation (Variables|Default|Getitem_dropper1) "/Game/Portal2Content/models/Dropper/item_dropper_Anim_item_dropper_qc_skeleton_item_dropper_open.item_dropper_Anim_item_dropper_qc_skeleton_item_dropper_open" false)
      (Audio|PlaySoundatLocation "/Game/Portal2Content/sounds/buttons/dropper_iris_open_01.dropper_iris_open_01" (Transformation|GetWorldLocation (Variables|Default|GetBox)) "0, 0, 0" 0.1 1.0 0.0 "/Game/Portal2Content/sounds/SA_Default.SA_Default" 0 0 0)
      (Utilities|FlowControl|Delay 0.75)
      (Collision|SetCollisionEnabled (Variables|Default|GetBox) "NoCollision")
      (Variables|Default|SetCanClose true))))

(event EventBeginPlay
  (Game|SpawnActorfromClass (Variables|Default|GetPropToSpawn_0) (Math|Transform|MakeTransform (Transformation|GetWorldLocation (Variables|Default|GetDefaultSceneRoot)) "0, 0, 0" "1.000000,1.000000,1.000000") "AlwaysSpawn" "MultiplyWithRoot" 0 0))

(event EventActivate
  (params (Investigator :type Actor%20Object%20Reference))
  (CallFunction|DropItem))

(fn ConstructionScript)