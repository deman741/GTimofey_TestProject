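; BP_Button01 is an interactable push button that sends an activate or deactivate message to its ParentedActor, as chosen by SendDeactivate.
; Interact hides the help widget shown by ViewHelp, then plays the press animation and sound, optionally adding a ticking cue and StartTimed delay before messaging.
; A DoOnce blocks repeat presses until the button pops back up shortly after the message.
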(event Custom|ViewHelp
  (Rendering|SetVisibility (Variables|Default|GetWidget) true false))

(event EventBeginPlay)

(event Collision|EventActorBeginOverlap
  (params (OtherActor :type Actor%20Object%20Reference)))

(event EventTick
  (params (DeltaSeconds :type Float%20%28single-precision%29)))

(event EventInteract
  (bind _parentedactor (Variables|Default|GetParentedActor))
  (bind _box (Variables|Default|GetBox))
  (bind _button01 (Variables|Default|Getbutton01))
  (Rendering|SetVisibility (Variables|Default|GetWidget) false false)
  (Utilities|FlowControl|DoOnce false :!label _label
    (:Completed
      (Components|Animation|PlayAnimation _button01 "/Game/Portal2Content/models/Button01/button01_Anim_switch001_qc_skeleton_down.button01_Anim_switch001_qc_skeleton_down" false)
      (Audio|PlaySoundatLocation "/Game/Portal2Content/sounds/buttons/button_synth_positive_01.button_synth_positive_01" (Transformation|GetWorldLocation _box) "0, 0, 0" 0.2 1.0 0.0 "/Game/Portal2Content/sounds/SA_Default.SA_Default" 0 0 0)
      (if (Variables|Default|GetStartTimed)
        (Audio|PlaySoundatLocation "/Game/Sounds/ui/synth_tick_tock_01_Cue.synth_tick_tock_01_Cue" (Transformation|GetWorldLocation (Variables|Default|GetBox)) "0, 0, 0" 1.0 1.0 0.0 0 0 0 0)
        (Utilities|FlowControl|Delay (Math|Conversions|ToFloat(Integer) (Variables|Default|GetStartOffsetSec))))
      (if (Variables|Default|GetSendDeactivate?)
        (Class|BPIButtonsInteract|Deactivate(Message) _parentedactor self)
        (else
          (Class|BPIButtonsInteract|Activate(Message) _parentedactor self)))
      (Utilities|FlowControl|Delay 0.8)
      (Components|Animation|PlayAnimation _button01 "/Game/Portal2Content/models/Button01/button01_Anim_switch001_qc_skeleton_up.button01_Anim_switch001_qc_skeleton_up" false)
      (Audio|PlaySoundatLocation "/Game/Portal2Content/sounds/buttons/button_synth_negative_02.button_synth_negative_02" (Transformation|GetWorldLocation _box) "0, 0, 0" 0.2 1.0 0.0 "/Game/Portal2Content/sounds/SA_Default.SA_Default" 0 0 0)
      (goto _label Reset))))

(fn ConstructionScript)