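; BP_tractor_beam_emitter is a tractor beam that drags physics props entering its Box trigger.
; A PullIn flag selects the beam core material in the Construction Script and the target: the emitter mesh when true, the EndPoint otherwise.
; On overlap, BP_PhysicProp components move there via MoveComponentTo, which re-triggers itself on completion.
; The file has no end-overlap logic to stop that loop.
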(event OnComponentBeginOverlap(Box)
  (params (OverlappedComponent :type Primitive%20Component%20Object%20Reference) (OtherActor :type Actor%20Object%20Reference) (OtherComp :type Primitive%20Component%20Object%20Reference) (OtherBodyIndex :type Integer) (bFromSweep :type Boolean) (SweepResult :type Hit%20Result%20Structure%20%28by%20ref%29))
  (Utilities|Casting|CastToBP_PhysicProp OtherActor)
  (if (Variables|Default|GetPullIn?)
    (Components|MoveComponentTo OtherComp (Transformation|GetWorldLocation (Variables|Default|Gettractor_beam_emitter1)) "0, 0, 0" false false 4.0 false :!label _label)
    (goto _label)
    (else
      (Components|MoveComponentTo OtherComp (Transformation|GetWorldLocation (Variables|Default|GetEndPoint)) "0, 0, 0" false false 4.0 false :!label _label_2)
      (goto _label_2))))

(event EventBeginPlay
  (if (Variables|Default|GetPullIn?)
    _))

(event Collision|EventActorBeginOverlap
  (params (OtherActor :type Actor%20Object%20Reference)))

(event EventTick
  (params (DeltaSeconds :type Float%20%28single-precision%29)))

(fn ConstructionScript
  (bind _cylinder (Variables|Default|GetCylinder))
  (if (Variables|Default|GetPullIn?)
    (Rendering|Material|SetMaterial _cylinder 0 "/Game/Portal2Content/models/tractor_beam_emitter/tractor_beam_core_Mat1.tractor_beam_core_Mat1")
    (else
      (Rendering|Material|SetMaterial _cylinder 0 "/Game/Portal2Content/models/tractor_beam_emitter/tractor_beam_core_Mat.tractor_beam_core_Mat"))))