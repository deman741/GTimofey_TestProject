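; Puzzle door that opens and closes when activated or deactivated, requiring one activator or, with TwoActivators, both a box and a ball socket.
; Indicator cube materials track each socket and double as the both-active check, which also plays a one-time GLaDOS line.
; Opening and closing play animation and sound, then toggle the blocking box's collision.
; A player overlapping Box1 closes an opened door, and BeginPlay registers it with a parent BP_ColorPuzzle.
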(event OnComponentBeginOverlap(Box1)
  (params (OverlappedComponent :type Primitive%20Component%20Object%20Reference) (OtherActor :type Actor%20Object%20Reference) (OtherComp :type Primitive%20Component%20Object%20Reference) (OtherBodyIndex :type Integer) (bFromSweep :type Boolean) (SweepResult :type Hit%20Result%20Structure%20%28by%20ref%29))
  (bind _box (Variables|Default|GetBox))
  (Utilities|Casting|CastToBP_Player OtherActor)
  (if (Variables|Default|GetOpened?)
    (Components|Animation|PlayAnimation (Variables|Default|Getdoor) "/Game/Portal2Content/models/Door/door_Anim_portal_door_combined_model_skeleton_close.door_Anim_portal_door_combined_model_skeleton_close" false)
    (Audio|PlaySoundatLocation "/Game/Portal2Content/sounds/doors/door_round_blue_close_01.door_round_blue_close_01" (Transformation|GetWorldLocation _box) "0, 0, 0" 0.5 1.0 0.0 "/Game/Portal2Content/sounds/SA_Default.SA_Default" 0 0 0)
    (Utilities|FlowControl|Delay 0.3)
    (Collision|SetCollisionEnabled _box "QueryAndPhysics")
    (Variables|Default|SetOpened? false)))

(event EventBeginPlay
  (bind _asbp_color_puzzle (Utilities|Casting|CastToBP_ColorPuzzle (Variables|Default|GetParentedActor)))
  (Variables|/Game/Actors/BP_ColorPuzzle.BP_ColorPuzzle_C|SetDoorActor _asbp_color_puzzle self))

(event EventActivate
  (params (Investigator :type Actor%20Object%20Reference))
  (bind _box (Variables|Default|GetBox))
  (bind _cube3 (Variables|Default|GetCube3))
  (bind _cube1 (Variables|Default|GetCube1))
  (if (Variables|Default|GetTwoActivators?)
    (Utilities|FlowControl|Delay 0.2)
    (Utilities|FlowControl|Sequence
      (:then_0
        (bind _asbp_box_socket (Utilities|Casting|CastToBP_BoxSocket Investigator))
        (Rendering|Material|SetMaterial _cube1 0 "/Game/Portal2Content/signage/indicator_checked_color_Mat.indicator_checked_color_Mat"))
      (:then_1
        (bind _asbp_ball_socket (Utilities|Casting|CastToBP_BallSocket Investigator))
        (Rendering|Material|SetMaterial _cube3 0 "/Game/Portal2Content/signage/indicator_checked_color_Mat.indicator_checked_color_Mat")))
    (if (== (== (Rendering|Material|GetMaterial _cube1 0) "/Game/Portal2Content/signage/indicator_checked_color_Mat.indicator_checked_color_Mat") (== (Rendering|Material|GetMaterial _cube3 0) "/Game/Portal2Content/signage/indicator_checked_color_Mat.indicator_checked_color_Mat"))
      (Variables|Default|SetOpened? false)
      (Utilities|FlowControl|Sequence
        (:then_0
          (Utilities|FlowControl|DoOnce false
            (:Completed
              (bind _asbp_player (Utilities|Casting|CastToBP_Player (Game|GetPlayerCharacter 0)))
              (Audio|Components|Audio|SetSound (Variables|/Game/Characters/Player/BP_Player.BP_Player_C|GetgladosVO _asbp_player) "/Game/Sounds/Glados/coop_test_chamber_oneplayer37.coop_test_chamber_oneplayer37")
              (Audio|Components|Audio|Play (Variables|/Game/Characters/Player/BP_Player.BP_Player_C|GetgladosVO _asbp_player) 0.0))))
        (:then_1
          (Utilities|FlowControl|Delay 0.1)
          (Components|Animation|PlayAnimation (Variables|Default|Getdoor) "/Game/Portal2Content/models/Door/door_Anim_portal_door_combined_model_skeleton_open.door_Anim_portal_door_combined_model_skeleton_open" false :!label _label)
          (Audio|PlaySoundatLocation "/Game/Portal2Content/sounds/doors/door_round_blue_unlock_01.door_round_blue_unlock_01" (Transformation|GetWorldLocation _box) "0, 0, 0" 0.5 1.0 0.0 "/Game/Portal2Content/sounds/SA_Default.SA_Default" 0 0 0)
          (Utilities|FlowControl|Delay 0.77)
          (Collision|SetCollisionEnabled _box "NoCollision")
          (Variables|Default|SetOpened? true))))
    (else
      (Rendering|Material|SetMaterial (Variables|Default|GetCube1) 0 "/Game/Portal2Content/signage/indicator_checked_color_Mat.indicator_checked_color_Mat")
      (goto _label))))

(event EventDeactivate
  (params (Investigator :type Actor%20Object%20Reference))
  (bind _box (Variables|Default|GetBox))
  (if (Variables|Default|GetTwoActivators?)
    (Utilities|FlowControl|Sequence
      (:then_0
        (bind _asbp_box_socket (Utilities|Casting|CastToBP_BoxSocket Investigator))
        (Rendering|Material|SetMaterial (Variables|Default|GetCube1) 0 "/Game/Portal2Content/signage/indicator_unchecked_color_Mat.indicator_unchecked_color_Mat"))
      (:then_1
        (bind _asbp_ball_socket (Utilities|Casting|CastToBP_BallSocket Investigator))
        (Rendering|Material|SetMaterial (Variables|Default|GetCube3) 0 "/Game/Portal2Content/signage/indicator_unchecked_color_Mat.indicator_unchecked_color_Mat")))
    (if (not (or (Variables|/Game/Actors/BP_BoxSocket.BP_BoxSocket_C|GetBoxSocketActivated _asbp_box_socket) (Variables|/Game/Actors/BP_BallSocket.BP_BallSocket_C|GetBallSocketActivated _asbp_ball_socket)))
      (if (Variables|Default|GetOpened?)
        (Utilities|FlowControl|Delay 0.1)
        (Components|Animation|PlayAnimation (Variables|Default|Getdoor) "/Game/Portal2Content/models/Door/door_Anim_portal_door_combined_model_skeleton_close.door_Anim_portal_door_combined_model_skeleton_close" false :!label _label)
        (Audio|PlaySoundatLocation "/Game/Portal2Content/sounds/doors/door_round_blue_close_01.door_round_blue_close_01" (Transformation|GetWorldLocation _box) "0, 0, 0" 0.5 1.0 0.0 "/Game/Portal2Content/sounds/SA_Default.SA_Default" 0 0 0)
        (Utilities|FlowControl|Delay 0.3)
        (Collision|SetCollisionEnabled _box "QueryAndPhysics")
        (Variables|Default|SetOpened? false)))
    (else
      (Rendering|Material|SetMaterial (Variables|Default|GetCube1) 0 "/Game/Portal2Content/signage/indicator_unchecked_color_Mat.indicator_unchecked_color_Mat")
      (goto _label))))

(event EventTick
  (params (DeltaSeconds :type Float%20%28single-precision%29)))

(fn ConstructionScript
  (bind _cube2 (Variables|Default|GetCube2))
  (if (Variables|Default|GetTwoActivators?)
    (Rendering|SetVisibility _cube2 true true)
    (else
      (Rendering|SetVisibility _cube2 false true))))