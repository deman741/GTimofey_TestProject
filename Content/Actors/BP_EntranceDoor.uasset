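; An entrance door actor that opens when the player enters its Sphere trigger and closes when the player leaves.
; Overlap events filtered to BP_Player play the open or close animation on the Door component, with an attenuated sound at the Box location.
; After a short delay in each case, the Box's collision is disabled on opening or set to physics-only on closing.
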(event OnComponentBeginOverlap(Sphere)
  (params (OverlappedComponent :type Primitive%20Component%20Object%20Reference) (OtherActor :type Actor%20Object%20Reference) (OtherComp :type Primitive%20Component%20Object%20Reference) (OtherBodyIndex :type Integer) (bFromSweep :type Boolean) (SweepResult :type Hit%20Result%20Structure%20%28by%20ref%29))
  (bind _box (Variables|Default|GetBox))
  (Utilities|Casting|CastToBP_Player OtherActor)
  (Components|Animation|PlayAnimation (Variables|Default|Getdoor) "/Game/Portal2Content/models/Door/door_Anim_portal_door_combined_model_skeleton_open.door_Anim_portal_door_combined_model_skeleton_open" false)
  (Audio|PlaySoundatLocation "/Game/Portal2Content/sounds/doors/door_round_blue_unlock_01.door_round_blue_unlock_01" (Transformation|GetWorldLocation _box) "0, 0, 0" 0.5 1.0 0.0 "/Game/Portal2Content/sounds/SA_Default.SA_Default" 0 0 0)
  (Utilities|FlowControl|Delay 0.77)
  (Collision|SetCollisionEnabled _box "NoCollision"))

(event OnComponentEndOverlap(Sphere)
  (params (OverlappedComponent :type Primitive%20Component%20Object%20Reference) (OtherActor :type Actor%20Object%20Reference) (OtherComp :type Primitive%20Component%20Object%20Reference) (OtherBodyIndex :type Integer))
  (bind _box (Variables|Default|GetBox))
  (Utilities|Casting|CastToBP_Player OtherActor)
  (Components|Animation|PlayAnimation (Variables|Default|Getdoor) "/Game/Portal2Content/models/Door/door_Anim_portal_door_combined_model_skeleton_close.door_Anim_portal_door_combined_model_skeleton_close" false)
  (Audio|PlaySoundatLocation "/Game/Portal2Content/sounds/doors/door_round_blue_close_01.door_round_blue_close_01" (Transformation|GetWorldLocation _box) "0, 0, 0" 0.5 1.0 0.0 "/Game/Portal2Content/sounds/SA_Default.SA_Default" 0 0 0)
  (Utilities|FlowControl|Delay 0.3)
  (Collision|SetCollisionEnabled _box "PhysicsOnly"))

(event EventBeginPlay)

(event Collision|EventActorBeginOverlap
  (params (OtherActor :type Actor%20Object%20Reference)))

(event EventTick
  (params (DeltaSeconds :type Float%20%28single-precision%29)))

(fn ConstructionScript)