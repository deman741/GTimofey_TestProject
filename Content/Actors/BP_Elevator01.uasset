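; Elevator actor that moves its Arm128 component between start and end locations when the player enters its trigger, with audio for the motion.
; Box1 overlaps drive a DoOnce-gated FlipFlop of MoveComponentTo calls and re-arm a second DoOnce, which Box2 fires to stop the move and return the arm to start.
; Separate Activate and Deactivate events play or reverse a Timeline that nudges the arm along Y, with direction set by the Finished flag.
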(event OnComponentBeginOverlap(Box1)
  (params (OverlappedComponent :type Primitive%20Component%20Object%20Reference) (OtherActor :type Actor%20Object%20Reference) (OtherComp :type Primitive%20Component%20Object%20Reference) (OtherBodyIndex :type Integer) (bFromSweep :type Boolean) (SweepResult :type Hit%20Result%20Structure%20%28by%20ref%29))
  (bind _arm128 (Variables|Default|Getarm128))
  (bind _arm128_2 (Variables|Default|Getarm128))
  (bind _audio (Variables|Default|GetAudio))
  (bind _relativerotation (Variables|/Script/Engine.SceneComponent|GetRelativeRotation _arm128_2))
  (Utilities|Casting|CastToBP_Player OtherActor)
  (Utilities|FlowControl|Sequence
    (:then_0
      (Utilities|FlowControl|DoOnce false :!label _label
        (:Completed
          (Utilities|FlowControl|FlipFlop :!label _label_2
            (:A
              (Audio|Components|Audio|Play _audio 0.0)
              (Components|MoveComponentTo _arm128 (Variables|Default|GetEndLoc) _relativerotation false false 4.0 false)
              (Variables|Default|SetFinished? true)
              (Audio|Components|Audio|Stop (Variables|Default|GetAudio))
              (Utilities|FlowControl|Delay 0.2)
              (goto _label Reset))
            (:B
              (if (Utilities|Operators|EqualEqual (Variables|/Script/Engine.SceneComponent|GetRelativeLocation (Variables|Default|Getarm128)) (Variables|Default|GetStartLoc) 0.0)
                (goto _label_2)
                (else
                  (Audio|Components|Audio|Play _audio 0.0)
                  (Components|MoveComponentTo _arm128 (Variables|Default|GetStartLoc) _relativerotation false false 3.0 false)
                  (Audio|Components|Audio|Stop (Variables|Default|GetAudio))
                  (Variables|Default|SetFinished? true)
                  (goto _label Reset))))))))
    (:then_1
      (Utilities|FlowControl|DoOnce true) ; enters at Reset
    )))

(event OnComponentBeginOverlap(Box2)
  (params (OverlappedComponent :type Primitive%20Component%20Object%20Reference) (OtherActor :type Actor%20Object%20Reference) (OtherComp :type Primitive%20Component%20Object%20Reference) (OtherBodyIndex :type Integer) (bFromSweep :type Boolean) (SweepResult :type Hit%20Result%20Structure%20%28by%20ref%29))
  (bind _arm128 (Variables|Default|Getarm128))
  (bind _arm128_2 (Variables|Default|Getarm128))
  (bind _audio (Variables|Default|GetAudio))
  (bind _relativerotation (Variables|/Script/Engine.SceneComponent|GetRelativeRotation _arm128_2))
  (Utilities|Casting|CastToBP_Player OtherActor)
  (Utilities|FlowControl|DoOnce true
    (:Completed
      (Utilities|FlowControl|Sequence
        (:then_0
          (Components|MoveComponentTo _arm128 (Variables|Default|GetEndLoc) _relativerotation false false 4.0 false) ; enters at Stop
        )
        (:then_1
          (Audio|Components|Audio|Play _audio 0.0)
          (Components|MoveComponentTo _arm128 (Variables|Default|GetStartLoc) _relativerotation false false 3.0 false)
          (Audio|Components|Audio|Stop (Variables|Default|GetAudio))
          (Variables|Default|SetFinished? true)
          (Utilities|FlowControl|DoOnce false) ; enters at Reset
        )))))

(event EventBeginPlay
  (Audio|Components|Audio|Stop (Variables|Default|GetAudio)))

(event Collision|EventActorBeginOverlap
  (params (OtherActor :type Actor%20Object%20Reference)))

(event EventTick
  (params (DeltaSeconds :type Float%20%28single-precision%29)))

(event EventActivate
  (params (Investigator :type Actor%20Object%20Reference))
  (Components|Timeline|SetPlayRate (Variables|Default|GetTimeline) (Variables|Default|GetNew%20Rate))
  (Audio|Components|Audio|Play (Variables|Default|GetAudio) 0.0)
  (bind _newtrack_0 (Timeline|Timeline Play)
    (:Update
      (if (Variables|Default|GetFinished?)
        (Transformation|AddLocalOffset (Variables|Default|Getarm128) "0.000000,6.000000,0.000000" false false)
        (else
          (Transformation|AddLocalOffset (Variables|Default|Getarm128) "0.000000,-1.600000,0.000000" false false))))
    (:Finished
      (Audio|Components|Audio|Stop (Variables|Default|GetAudio))
      (if (Variables|Default|GetFinished?)
        (Variables|Default|SetFinished? false)
        (else
          (Variables|Default|SetFinished? true))))))

(event EventDeactivate
  (params (Investigator :type Actor%20Object%20Reference))
  (Components|Timeline|SetPlayRate (Variables|Default|GetTimeline) (Variables|Default|GetNew%20Rate))
  (Audio|Components|Audio|Play (Variables|Default|GetAudio) 0.0)
  (Variables|Default|SetFinished? false)
  (bind _newtrack_0 (Timeline|Timeline ReverseFromEnd)
    (:Update
      (if (Variables|Default|GetFinished?)
        (Transformation|AddLocalOffset (Variables|Default|Getarm128) "0.000000,6.000000,0.000000" false false)
        (else
          (Transformation|AddLocalOffset (Variables|Default|Getarm128) "0.000000,-1.600000,0.000000" false false))))
    (:Finished
      (Audio|Components|Audio|Stop (Variables|Default|GetAudio))
      (if (Variables|Default|GetFinished?)
        (Variables|Default|SetFinished? false)
        (else
          (Variables|Default|SetFinished? true))))))

(fn ConstructionScript)