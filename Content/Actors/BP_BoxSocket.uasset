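; BP_BoxSocket is a Portal-style floor socket that activates when a BP_MetalBox sits in it and deactivates when the box leaves.
; Box2 overlaps drive delayed socket animation, material, sound and box skin changes, and set BoxSocketActivated.
; Each change notifies ParentedActor through Activate and Deactivate messages.
; A BP_MetalBall entering instead triggers a GLaDOS voice line on the player, gated by a DoOnce that resets after a delay.
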(event OnComponentBeginOverlap(Box2)
  (params (OverlappedComponent :type Primitive%20Component%20Object%20Reference) (OtherActor :type Actor%20Object%20Reference) (OtherComp :type Primitive%20Component%20Object%20Reference) (OtherBodyIndex :type Integer) (bFromSweep :type Boolean) (SweepResult :type Hit%20Result%20Structure%20%28by%20ref%29))
  (Utilities|FlowControl|Sequence
    (:then_0
      (Utilities|Casting|CastToBP_MetalBox OtherActor)
      (Utilities|FlowControl|RetriggerableDelay 0.2)
      (Components|Animation|PlayAnimation (Variables|Default|Getbox_socket1) "/Game/Portal2Content/models/box_socket/box_socket_Anim_box_socket_reference_skeleton_down.box_socket_Anim_box_socket_reference_skeleton_down" false)
      (Rendering|Material|SetMaterial (Variables|Default|Getbox_socket1) 0 "/Game/Portal2Content/models/box_socket/box_socket2.box_socket2")
      (Variables|Default|SetBoxSocketActivated true)
      (Class|BPIButtonsInteract|Activate(Message) (Variables|Default|GetParentedActor) self)
      (Audio|PlaySoundatLocation "/Game/Portal2Content/sounds/buttons/portal_button_down_01.portal_button_down_01" (Transformation|GetWorldLocation (Variables|Default|GetBox3)) "0, 0, 0" 0.05 1.0 0.0 0 0 0 0)
      (bind _asbp_metal_box (Utilities|Casting|CastToBP_MetalBox OtherActor))
      (Default|ChangeSkin _asbp_metal_box))
    (:then_1
      (Utilities|Casting|CastToBP_MetalBall OtherActor)
      (Utilities|FlowControl|DoOnce false :!label _label
        (:Completed
          (bind _asbp_player (Utilities|Casting|CastToBP_Player (Game|GetPlayerCharacter 0)))
          (Audio|Components|Audio|SetSound (Variables|/Game/Characters/Player/BP_Player.BP_Player_C|GetgladosVO _asbp_player) "/Game/Sounds/Glados/mp_coop_startdeath02_Cue.mp_coop_startdeath02_Cue")
          (Audio|Components|Audio|Play (Variables|/Game/Characters/Player/BP_Player.BP_Player_C|GetgladosVO _asbp_player) 0.0)
          (Utilities|FlowControl|Delay 1.5)
          (goto _label Reset))))))

(event OnComponentEndOverlap(Box2)
  (params (OverlappedComponent :type Primitive%20Component%20Object%20Reference) (OtherActor :type Actor%20Object%20Reference) (OtherComp :type Primitive%20Component%20Object%20Reference) (OtherBodyIndex :type Integer))
  (Utilities|Casting|CastToBP_MetalBox OtherActor)
  (Utilities|FlowControl|Delay 0.3)
  (Components|Animation|PlayAnimation (Variables|Default|Getbox_socket1) "/Game/Portal2Content/models/box_socket/box_socket_Anim_box_socket_reference_skeleton_up.box_socket_Anim_box_socket_reference_skeleton_up" false)
  (Rendering|Material|SetMaterial (Variables|Default|Getbox_socket1) 0 "/Game/Portal2Content/models/box_socket/box_socket.box_socket")
  (Variables|Default|SetBoxSocketActivated false)
  (Audio|PlaySoundatLocation "/Game/Portal2Content/sounds/buttons/portal_button_up_01.portal_button_up_01" (Transformation|GetWorldLocation (Variables|Default|GetBox3)) "0, 0, 0" 0.05 1.0 0.0 0 0 0 0)
  (Class|BPIButtonsInteract|Deactivate(Message) (Variables|Default|GetParentedActor) self)
  (Default|ReturnSkin (stale OnComponentBeginOverlap(Box2) _asbp_metal_box)))

(event EventBeginPlay)

(event Collision|EventActorBeginOverlap
  (params (OtherActor :type Actor%20Object%20Reference)))

(event EventTick
  (params (DeltaSeconds :type Float%20%28single-precision%29)))

(fn ConstructionScript)