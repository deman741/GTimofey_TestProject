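; BP_BallSocket is a Portal-style socket button that a BP_MetalBall activates.
; Box2 overlaps drive it: after short delays it animates, swaps material, plays a sound and toggles the ball's skin.
; It also sets its activated flag and sends Activate or Deactivate messages to ParentedActor.
; A BP_MetalBox overlap instead plays a GLaDOS voice line on the player, gated by a resetting DoOnce.
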(event OnComponentBeginOverlap(Box2)
  (params (OverlappedComponent :type Primitive%20Component%20Object%20Reference) (OtherActor :type Actor%20Object%20Reference) (OtherComp :type Primitive%20Component%20Object%20Reference) (OtherBodyIndex :type Integer) (bFromSweep :type Boolean) (SweepResult :type Hit%20Result%20Structure%20%28by%20ref%29))
  (Utilities|FlowControl|Sequence
    (:then_0
      (Utilities|Casting|CastToBP_MetalBox OtherActor)
      (Utilities|FlowControl|DoOnce false :!label _label
        (:Completed
          (bind _asbp_player (Utilities|Casting|CastToBP_Player (Game|GetPlayerCharacter 0)))
          (Audio|Components|Audio|SetSound (Variables|/Game/Characters/Player/BP_Player.BP_Player_C|GetgladosVO _asbp_player) "/Game/Sounds/Glados/mp_coop_startdeath02_Cue.mp_coop_startdeath02_Cue")
          (Audio|Components|Audio|Play (Variables|/Game/Characters/Player/BP_Player.BP_Player_C|GetgladosVO _asbp_player) 0.0)
          (Utilities|FlowControl|Delay 1.5)
          (goto _label Reset))))
    (:then_1
      (Utilities|Casting|CastToBP_MetalBall OtherActor)
      (Utilities|FlowControl|RetriggerableDelay 0.2)
      (Components|Animation|PlayAnimation (Variables|Default|Getball_socket) "/Game/Portal2Content/models/ball_socket/ball_socket_Anim.ball_socket_Anim" false)
      (Rendering|Material|SetMaterial (Variables|Default|Getball_socket) 0 "/Game/Portal2Content/models/ball_socket/ball_button1.ball_button1")
      (Variables|Default|SetBallSocketActivated true)
      (Class|BPIButtonsInteract|Activate(Message) (Variables|Default|GetParentedActor) self)
      (Audio|PlaySoundatLocation "/Game/Portal2Content/sounds/buttons/portal_button_down_01.portal_button_down_01" (Transformation|GetWorldLocation (Variables|Default|GetBox3)) "0, 0, 0" 0.05 1.0 0.0 0 0 0 0)
      (bind _asbp_metal_ball (Utilities|Casting|CastToBP_MetalBall OtherActor))
      (Default|ChangeSkin _asbp_metal_ball))))

(event OnComponentEndOverlap(Box2)
  (params (OverlappedComponent :type Primitive%20Component%20Object%20Reference) (OtherActor :type Actor%20Object%20Reference) (OtherComp :type Primitive%20Component%20Object%20Reference) (OtherBodyIndex :type Integer))
  (Utilities|Casting|CastToBP_MetalBall OtherActor)
  (Utilities|FlowControl|Delay 0.3)
  (Components|Animation|PlayAnimation (Variables|Default|Getball_socket) "/Game/Portal2Content/models/Button02/button02_Anim_portal_button_qc_skeleton_up.button02_Anim_portal_button_qc_skeleton_up" false)
  (Rendering|Material|SetMaterial (Variables|Default|Getball_socket) 0 "/Game/Portal2Content/models/ball_socket/ball_button.ball_button")
  (Variables|Default|SetBallSocketActivated false)
  (Audio|PlaySoundatLocation "/Game/Portal2Content/sounds/buttons/portal_button_up_01.portal_button_up_01" (Transformation|GetWorldLocation (Variables|Default|GetBox3)) "0, 0, 0" 0.05 1.0 0.0 0 0 0 0)
  (Class|BPIButtonsInteract|Deactivate(Message) (Variables|Default|GetParentedActor) self)
  (Default|ReturnSkin (stale OnComponentBeginOverlap(Box2) _asbp_metal_ball)))

(event EventBeginPlay)

(event Collision|EventActorBeginOverlap
  (params (OtherActor :type Actor%20Object%20Reference)))

(event EventTick
  (params (DeltaSeconds :type Float%20%28single-precision%29)))

(fn ConstructionScript)