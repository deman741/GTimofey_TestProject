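; BP_Arm is an animated arm actor with configurable material and animation.
; The construction script applies both to the Arm64 mesh without playing, and hides the Cube unless UseBlackMat is set.
; With StartWithBeginPlay, the animation loops immediately from BeginPlay.
; Otherwise, the StartAnim event waits an offset, plays it once, then destroys the actor after DeadTime.
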(event Custom|StartAnim
  (Utilities|FlowControl|Delay (Variables|Default|GetStartAnimOffset))
  (Components|Animation|PlayAnimation (Variables|Default|Getarm64) (Variables|Default|GetAnimation) (Variables|Default|GetStartWithBeginPlay))
  (if (not (Variables|Default|GetStartWithBeginPlay))
    (Utilities|FlowControl|Delay (Variables|Default|GetDeadTime))
    (Actor|DestroyActor)))

(event EventBeginPlay
  (if (Variables|Default|GetStartWithBeginPlay)
    (Components|Animation|PlayAnimation (Variables|Default|Getarm64) (Variables|Default|GetAnimation) (Variables|Default|GetStartWithBeginPlay))
    (if (not (Variables|Default|GetStartWithBeginPlay))
      (Utilities|FlowControl|Delay (Variables|Default|GetDeadTime))
      (Actor|DestroyActor))))

(fn ConstructionScript
  (Rendering|Material|SetMaterial (Variables|Default|Getarm64) 0 (Variables|Default|GetMaterial))
  (Components|Animation|OverrideAnimationData (Variables|Default|Getarm64) (Variables|Default|GetAnimation) false false 0.0 1.0)
  (if (not (Variables|Default|GetUseBlackMat))
    (Rendering|SetVisibility (Variables|Default|GetCube) false false)))