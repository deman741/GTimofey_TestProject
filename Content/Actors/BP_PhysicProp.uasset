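; BP_PhysicProp is a physics prop, typed as box or ball, with swappable skins and impact sounds.
; ChangeSkin and ReturnSkin switch the mesh between an alternate and default material for its type.
; On hit, if upward velocity exceeds a small threshold, it plays an attenuated sound at the mesh, with volume scaled from X velocity only.
; A DoOnce reset after a short delay throttles repeated sounds.
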(event OnComponentHit(MeshProp)
  (params (HitComponent :type Primitive%20Component%20Object%20Reference) (OtherActor :type Actor%20Object%20Reference) (OtherComp :type Primitive%20Component%20Object%20Reference) (NormalImpulse :type Vector :default "0, 0, 0") (Hit :type Hit%20Result%20Structure%20%28by%20ref%29))
  (bind _returnvalue (Physics|GetPhysicsLinearVelocity (Variables|Default|GetMeshProp) "None"))
  (Math|Float|CompareFloat (.Z (Math|Vector|BreakVector _returnvalue)) 4.0
    (:>
      (Utilities|FlowControl|DoOnce false :!label _label
        (:Completed
          (Audio|PlaySoundatLocation (Variables|Default|GetSound) (Transformation|GetWorldLocation (Variables|Default|GetMeshProp)) "0, 0, 0" (Math|Float|Clamp(Float) (/ (Math|Vector|VectorLength (Math|Conversions|ToVector(Float) (.X (Math|Vector|BreakVector _returnvalue)))) 1.2e+03) 0.1) 1.0 0.0 "/Game/Portal2Content/sounds/SA_Default.SA_Default" 0 0 0)
          (Utilities|FlowControl|Delay 0.2)
          (goto _label Reset))))))

(event Custom|ChangeSkin
  (switch Utilities|FlowControl|Switch|SwitchonE_PhysicProps (Variables|Default|GetTypeOfProp)
    (:NewEnumerator0
      (Rendering|Material|SetMaterial (Variables|Default|GetMeshProp) 0 "/Game/Portal2Content/models/Box/metal_box1.metal_box1"))
    (:NewEnumerator1
      (Rendering|Material|SetMaterial (Variables|Default|GetMeshProp) 0 "/Game/Portal2Content/models/metalball/mp_ball1.mp_ball1"))))

(event Custom|ReturnSkin
  (switch Utilities|FlowControl|Switch|SwitchonE_PhysicProps (Variables|Default|GetTypeOfProp)
    (:NewEnumerator0
      (Rendering|Material|SetMaterial (Variables|Default|GetMeshProp) 0 "/Game/Portal2Content/models/Box/metal_box.metal_box"))
    (:NewEnumerator1
      (Rendering|Material|SetMaterial (Variables|Default|GetMeshProp) 0 "/Game/Portal2Content/models/metalball/mp_ball.mp_ball"))))

(event EventBeginPlay)

(event Collision|EventActorBeginOverlap
  (params (OtherActor :type Actor%20Object%20Reference)))

(event EventTick
  (params (DeltaSeconds :type Float%20%28single-precision%29)))

(fn ConstructionScript)