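; Color memory puzzle actor that flashes a timed color sequence and opens a linked door when the entered code matches.
; Activate appends each Investigator to CurrentCode, and Deactivate either plays the sequence or compares CurrentCode with Code.
; StartPazzle hardcodes the flash order separately from Code and toggles box collision around playback.
; Success triggers GLaDOS voice and DoorActor, while failure clears input, counts a player mistake and re-arms playback.
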(event Custom|StartPazzle
  (bind _g (Variables|Default|GetG))
  (bind _y (Variables|Default|GetY))
  (bind _b (Variables|Default|GetB))
  (bind _r (Variables|Default|GetR))
  (bind _y_2 (Variables|Default|GetY))
  (bind _duration (Variables|Default|GetDuration))
  (bind _duration_2 (Variables|Default|GetDuration))
  (bind _asbp_player (Utilities|Casting|CastToBP_Player (Game|GetPlayerCharacter 0)))
  (Audio|Components|Audio|SetSound (Variables|/Game/Characters/Player/BP_Player.BP_Player_C|GetgladosVO _asbp_player) "/Game/Sounds/Glados/coop_numbers13_Cue.coop_numbers13_Cue")
  (Audio|Components|Audio|Play (Variables|/Game/Characters/Player/BP_Player.BP_Player_C|GetgladosVO _asbp_player) 0.0)
  (Collision|SetCollisionEnabled (Variables|Default|GetBox1) "QueryAndPhysics")
  (Rendering|SetVisibility (Variables|Default|GetB) false false)
  (Utilities|FlowControl|Delay 3.0)
  (Rendering|SetVisibility _g true false)
  (Audio|PlaySound2D "/Game/Sounds/ui/menu_countdown.menu_countdown" 1.0 1.0 0.0 0 0)
  (Utilities|FlowControl|Delay _duration)
  (Rendering|SetVisibility _g false false)
  (Rendering|SetVisibility _y true false)
  (Audio|PlaySound2D "/Game/Sounds/ui/menu_countdown.menu_countdown" 1.0 1.0 0.0 0 0)
  (Utilities|FlowControl|Delay _duration)
  (Rendering|SetVisibility _y false false)
  (Rendering|SetVisibility _b true false)
  (Audio|PlaySound2D "/Game/Sounds/ui/menu_countdown.menu_countdown" 1.0 1.0 0.0 0 0)
  (Utilities|FlowControl|Delay _duration)
  (Rendering|SetVisibility _b false false)
  (Rendering|SetVisibility _r true false)
  (Audio|PlaySound2D "/Game/Sounds/ui/menu_countdown.menu_countdown" 1.0 1.0 0.0 0 0)
  (Utilities|FlowControl|Delay _duration_2)
  (Rendering|SetVisibility _r false false)
  (Rendering|SetVisibility _y_2 true false)
  (Audio|PlaySound2D "/Game/Sounds/ui/menu_countdown.menu_countdown" 1.0 1.0 0.0 0 0)
  (Utilities|FlowControl|Delay _duration_2)
  (Rendering|SetVisibility _y_2 false false)
  (Utilities|FlowControl|Delay 0.2)
  (Collision|SetCollisionEnabled (Variables|Default|GetBox1) "NoCollision")
  (Rendering|SetVisibility (Variables|Default|GetBox) false false)
  (Variables|Default|SetStartPazzle? false))

(event EventBeginPlay)

(event Collision|EventActorBeginOverlap
  (params (OtherActor :type Actor%20Object%20Reference)))

(event EventTick
  (params (DeltaSeconds :type Float%20%28single-precision%29)))

(event EventActivate
  (params (Investigator :type Actor%20Object%20Reference))
  (Utilities|Array|Add (Variables|Default|GetCurrentCode) Investigator))

(event EventDeactivate
  (params (Investigator :type Actor%20Object%20Reference))
  (if (Variables|Default|GetStartPazzle?)
    (CallFunction|StartPazzle)
    (elif (Utilities|Array|Identical (Variables|Default|GetCode) (Variables|Default|GetCurrentCode))
      (Collision|SetCollisionEnabled (Variables|Default|GetBox1) "QueryAndPhysics")
      (Components|Activation|SetActive (Variables|Default|GetAudio) true false)
      (bind _asbp_player (Utilities|Casting|CastToBP_Player (Game|GetPlayerCharacter 0)))
      (Audio|Components|Audio|SetSound (Variables|/Game/Characters/Player/BP_Player.BP_Player_C|GetgladosVO _asbp_player) "/Game/Sounds/Glados/mp_coop_wall_block03_Cue.mp_coop_wall_block03_Cue")
      (Utilities|FlowControl|Delay 1.0)
      (Audio|Components|Audio|Play (Variables|/Game/Characters/Player/BP_Player.BP_Player_C|GetgladosVO _asbp_player) 0.0)
      (Utilities|FlowControl|Delay 3.0)
      (Class|BPIButtonsInteract|Activate(Message) (Variables|Default|GetDoorActor))
      (else
        (Utilities|Array|Clear (Variables|Default|GetCurrentCode))
        (Variables|Default|SetStartPazzle? true)
        (bind _asbp_player_2 (Utilities|Casting|CastToBP_Player (Game|GetPlayerCharacter 0)))
        (Default|AddOnetoMistakes _asbp_player_2)
        (Utilities|FlowControl|Delay 4.0)
        (Audio|Components|Audio|SetSound (Variables|/Game/Characters/Player/BP_Player.BP_Player_C|GetgladosVO _asbp_player_2) "/Game/Sounds/Glados/faithplategarbage06.faithplategarbage06")
        (Audio|Components|Audio|Play (Variables|/Game/Characters/Player/BP_Player.BP_Player_C|GetgladosVO _asbp_player_2) 0.0)))))

(fn ConstructionScript)